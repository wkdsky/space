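; Mars chapter solar combiner cabinet that shows a burnt core being replaced when the unit is repaired.
; ApplyStoredState snaps door, core meshes and status light to the repaired or broken look from Active, on BeginPlay and on state changes.
; Runtime activation plays a MoveComponentTo sequence that opens the door, discards the burnt core, slides in the new one, closes up and turns the light green.
; A RepairAnimating flag blocks state snapping during the animation.
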(event Custom|OnStateChanged_0
  (params (bActive :type Boolean))
  (CallFunction|ApplyStoredState))

(event Custom|OnRuntimeActivated_0
  (params (bActive :type Boolean))
  (Variables|Default|SetRepairAnimating true)
  (Transformation|SetRelativeRotation (Variables|Default|GetCabinetDoor) "0,55,0" false false)
  (Transformation|SetRelativeRotation (Variables|Default|GetCoreBurntInSlot) "0,0,90" false false)
  (Transformation|SetRelativeLocation (Variables|Default|GetCoreBurntInSlot) "44,-45,95" false false)
  (Rendering|SetVisibility (Variables|Default|GetCoreBurntInSlot) true false)
  (Rendering|SetVisibility (Variables|Default|GetCoreInstalled) false false)
  (Rendering|SetVisibility (Variables|Default|GetCoreDiscarded) false false)
  (Rendering|Material|SetMaterial (Variables|Default|GetStatusLight) 0 "/Game/Space/Environment/MarsSystem/Chapter/Refined/M_MP_PowerRed.M_MP_PowerRed")
  (Components|MoveComponentTo (Variables|Default|GetCabinetDoor) "44,57,15" "0,105,0" true true 0.25 true)
  (Components|MoveComponentTo (Variables|Default|GetCoreBurntInSlot) "78,35,24" "90,25,0" true true 0.3 true)
  (Rendering|SetVisibility (Variables|Default|GetCoreBurntInSlot) false false)
  (Rendering|SetVisibility (Variables|Default|GetCoreDiscarded) true false)
  (Transformation|SetRelativeLocation (Variables|Default|GetCoreInstalled) "85,-45,95" false false)
  (Rendering|SetVisibility (Variables|Default|GetCoreInstalled) true false)
  (Components|MoveComponentTo (Variables|Default|GetCoreInstalled) "37,-45,95" "0,0,90" true true 0.4 true)
  (Components|MoveComponentTo (Variables|Default|GetCabinetDoor) "44,57,15" "0, 0, 0" true true 0.55 true)
  (Variables|Default|SetRepairAnimating false)
  (Rendering|Material|SetMaterial (Variables|Default|GetStatusLight) 0 "/Game/Space/Environment/MarsSystem/Chapter/Refined/M_MP_PowerGreen.M_MP_PowerGreen"))

(event EventBeginPlay
  (EventDispatchers|BindEventtoOnStateChanged (delegate Custom|OnStateChanged_0))
  (EventDispatchers|BindEventtoOnRuntimeActivated (delegate Custom|OnRuntimeActivated_0))
  (CallFunction|ApplyStoredState))

(fn ConstructionScript)

(fn ApplyStoredState
  (if (not (Variables|Default|GetRepairAnimating))
    (if (Variables|Default|GetbActive)
      (Transformation|SetRelativeRotation (Variables|Default|GetCabinetDoor) "0, 0, 0" false false)
      (Rendering|SetVisibility (Variables|Default|GetCoreBurntInSlot) false false)
      (Rendering|SetVisibility (Variables|Default|GetCoreInstalled) true false)
      (Rendering|SetVisibility (Variables|Default|GetCoreDiscarded) true false)
      (Transformation|SetRelativeLocation (Variables|Default|GetCoreBurntInSlot) "44,-45,95" false false)
      (Transformation|SetRelativeRotation (Variables|Default|GetCoreBurntInSlot) "0,0,90" false false)
      (Transformation|SetRelativeLocation (Variables|Default|GetCoreInstalled) "37,-45,95" false false)
      (Rendering|Material|SetMaterial (Variables|Default|GetStatusLight) 0 "/Game/Space/Environment/MarsSystem/Chapter/Refined/M_MP_PowerGreen.M_MP_PowerGreen")
      (else
        (Transformation|SetRelativeRotation (Variables|Default|GetCabinetDoor) "0,55,0" false false)
        (Rendering|SetVisibility (Variables|Default|GetCoreBurntInSlot) true false)
        (Rendering|SetVisibility (Variables|Default|GetCoreInstalled) false false)
        (Rendering|SetVisibility (Variables|Default|GetCoreDiscarded) false false)
        (Transformation|SetRelativeLocation (Variables|Default|GetCoreBurntInSlot) "44,-45,95" false false)
        (Transformation|SetRelativeRotation (Variables|Default|GetCoreBurntInSlot) "0,0,90" false false)
        (Transformation|SetRelativeLocation (Variables|Default|GetCoreInstalled) "37,-45,95" false false)
        (Rendering|Material|SetMaterial (Variables|Default|GetStatusLight) 0 "/Game/Space/Environment/MarsSystem/Chapter/Refined/M_MP_PowerRed.M_MP_PowerRed")))))